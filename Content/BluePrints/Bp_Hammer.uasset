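; Bp_Hammer is an actor that ends the game when something overlaps it, apparently as a goal pickup.
; One second after BeginPlay, it switches on overlap events for its Collision component.
; The first overlap, with no check on the other actor, destroys the DwarfSwordLv1 component and pauses the game.
; It then shows the WBP_GameFinished widget with the mouse cursor and UI-only input.
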(event `self.ReceiveBeginPlay`
  (`KismetSystemLibrary.Delay` 1.0)
  (set `PrimitiveComponent.bGenerateOverlapEvents` true (`self.Collision`)))

(event `self.Collision.OnComponentBeginOverlap`
  (params (OverlappedComponent :type "PrimitiveComponent Object Reference") (OtherActor :type "Actor Object Reference") (OtherComp :type "PrimitiveComponent Object Reference") (OtherBodyIndex :type Integer) (bFromSweep :type Boolean) (SweepResult :type "HitResult Structure (by ref)"))
  (bind _returnvalue (`GameplayStatics.GetPlayerController` 0))
  (`/Engine/EditorBlueprintResources/StandardMacros.DoOnce` false
    (:`Completed`
      (`ActorComponent.K2_DestroyComponent` (`self.dwarf_sword_lv1`))
      (`GameplayStatics.SetGamePaused` true)
      (bind _returnvalue_2 (`|CreateWidget` "/Game/BluePrints/WBP_GameFinished.WBP_GameFinished_C" _returnvalue))
      (`UserWidget.AddToViewport` _returnvalue_2 0)
      (set `PlayerController.bShowMouseCursor` true _returnvalue)
      (`WidgetBlueprintLibrary.SetInputMode_UIOnlyEx` _returnvalue _returnvalue_2))))

(fn `UserConstructionScript`)