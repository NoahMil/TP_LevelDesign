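; Door Blueprint that opens by sliding its mesh to a target location once all linked switches report solved.
; The Opening event checks every entry in Switchs via SolvedMessage, clearing SwitchStatus at the first unsolved one.
; A timeline lerps the mesh open, then after a short delay blends the view target back to the player character.
; CheckSwitchs never resets SwitchStatus to true, and its own Solved function always returns false.
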(event `/Game/BluePrints/Door/BI_Door.Opening`
  (`KismetSystemLibrary.PrintString` "Porte Débloquée")
  (bind _allswitchssolved (`self.CheckSwitchs`))
  (if _allswitchssolved
    (`self.DoorAnimation`)))

(event `DoorAnimation`
  (`KismetSystemLibrary.PrintString` "Ouverture")
  (bind (_direction _opentrack) (`Timeline|Timeline_open`)
    (:`Update`
      (`SceneComponent.K2_SetRelativeLocation` (`self.Door_Mesh`) (`KismetMathLibrary.VLerp` (0.0 0.0 0.0) (`self.Door_open_Location`) _opentrack) false false))
    (:`Finished`
      (`KismetSystemLibrary.Delay` 1.0)
      (`PlayerController.SetViewTargetWithBlend` (`GameplayStatics.GetPlayerController` 0) (`GameplayStatics.GetPlayerCharacter` 0) 0.0 "VTBlend_Linear" 0.0 false))))

(fn `CheckSwitchs`
  (returns (AllSwitchsSolved :type Boolean))
  (locals (SwitchStatus :type Boolean :default true))
  (for _array_element (`self.Switchs`)
    (bind _istrigger (message `/Game/BluePrints/Door/BI_Door.Solved` _array_element))
    (if (not _istrigger)
      (set `local.SwitchStatus` false)
      (break)))
  (return (`local.SwitchStatus`)))

(fn `Solved`
  (returns (IsTrigger :type Boolean))
  (return false))

(fn `UserConstructionScript`)