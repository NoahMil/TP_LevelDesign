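; Puzzle door that slides open once at least two of its linked switches report solved.
; Opening recounts the switches through their SolvedMessage, turning the two door lights green as the count rises.
; At two or more, a timeline lerps the door to its open location.
; Either outcome then waits briefly, blends the view back to the player character and calls EnableInput on it.
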(event `self.Opening`
  (`KismetSystemLibrary.PrintString` "Porte Débloquée")
  (`self.CheckSwitchs`)
  (if (>= (`self.ActivatedSwitchCount `) 2)
    (`self.DoorAnimation`)
    (else
      (`KismetSystemLibrary.Delay` 1.0)
      (`PlayerController.SetViewTargetWithBlend` (`GameplayStatics.GetPlayerController` 0) (`GameplayStatics.GetPlayerCharacter` 0) 0.0 "VTBlend_Linear" 0.0 false)
      (`self.EnableInput` (`GameplayStatics.GetPlayerCharacter` 0) null))))

(event `DoorAnimation`
  (bind _returnvalue (`GameplayStatics.GetPlayerController` 0))
  (`KismetSystemLibrary.PrintString` "Ouverture")
  (bind (_direction _opentrack) (`Timeline|Timeline_open`)
    (:`Update`
      (`SceneComponent.K2_SetRelativeLocation` (`self.NSM_PuzzleDoor`) (`KismetMathLibrary.VLerp` (0.0 0.0 0.0) (`self.Door_open_Location`) _opentrack) false false))
    (:`Finished`
      (`KismetSystemLibrary.Delay` 1.0)
      (`PlayerController.SetViewTargetWithBlend` _returnvalue (`GameplayStatics.GetPlayerCharacter` 0) 0.0 "VTBlend_Linear" 0.0 false)
      (`self.EnableInput` (`GameplayStatics.GetPlayerCharacter` 0) _returnvalue))))

(fn `CheckSwitchs`
  (locals (SwitchStatus :type Boolean :default true))
  (set `self.ActivatedSwitchCount ` 0)
  (for _array_element (`self.Switchs`)
    (bind _istrigger (message `/Game/BluePrints/Door/BI_Door.Solved` _array_element))
    (if _istrigger
      (set `self.ActivatedSwitchCount ` (+ (`self.ActivatedSwitchCount `) 1))))
  (if (>= (`self.ActivatedSwitchCount `) 1)
    (`PrimitiveComponent.SetMaterial` (`self.NSM_PuzzleDoor_Light_01`) 0 "/Game/Materials/M_Green.M_Green")
    (if (>= (`self.ActivatedSwitchCount `) 2)
      (`PrimitiveComponent.SetMaterial` (`self.NSM_PuzzleDoor_Light_02`) 0 "/Game/Materials/M_Green.M_Green")))
  (return))

(fn `Solved`
  (returns (IsTrigger :type Boolean))
  (return false))

(fn `UpdateLights`)

(fn `UserConstructionScript`)