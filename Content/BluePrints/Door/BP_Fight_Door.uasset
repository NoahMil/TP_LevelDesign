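; BP_Fight_Door is a door that slides open when its Opening event is called, then hands camera and control back to the player.
; DoorAnimation plays a timeline that lerps the NSMPuzzleDoor relative location from zero to DoorOpenLocation, with debug prints along the way.
; One second after it finishes, the view target returns to the player character and input is re-enabled.
; The Solved function is a stub returning false.
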(event `self.Opening`
  (`KismetSystemLibrary.PrintString` "Porte Débloquée")
  (`self.DoorAnimation`))

(event `DoorAnimation`
  (bind _returnvalue (`GameplayStatics.GetPlayerController` 0))
  (`KismetSystemLibrary.PrintString` "Ouverture")
  (bind (_direction _opentrack) (`Timeline|Timeline_open`)
    (:`Update`
      (`SceneComponent.K2_SetRelativeLocation` (`self.NSM_PuzzleDoor`) (`KismetMathLibrary.VLerp` (0.0 0.0 0.0) (`self.Door_open_Location`) _opentrack) false false))
    (:`Finished`
      (`KismetSystemLibrary.Delay` 1.0)
      (`PlayerController.SetViewTargetWithBlend` _returnvalue (`GameplayStatics.GetPlayerCharacter` 0) 0.0 "VTBlend_Linear" 0.0 false)
      (`self.EnableInput` (`GameplayStatics.GetPlayerCharacter` 0) _returnvalue))))

(fn `Solved`
  (returns (IsTrigger :type Boolean))
  (return false))

(fn `UserConstructionScript`)