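; BP_Switch is a switch that, when damaged, triggers its linked Door as part of a puzzle.
; An ApplyDamage event plays a timeline that slides the switch mesh along Y, then marks it solved and turns it green.
; It then blends the camera to the Door, disables player input and sends the Door an opening message.
; A Solved function exposes the state, while Opening is an empty stub.
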(event `/Game/Variant_Combat/Blueprints/BPI_Damageable.Apply Damage`
  (params (Damage :type "Float (double-precision)") (`Damage Causer` :type "Actor Object Reference") (`Damage Location` :type "Vector Structure") (`Damage Impulse` :type "Vector Structure"))
  (if (not (`self.IsSolved`))
    (bind (_direction _switcheffect) (`Timeline|Timeline_Switch`)
      (:`Update`
        (`SceneComponent.K2_SetRelativeLocation` (`self.Switch_Mesh`) (`KismetMathLibrary.MakeVector` 0.0 (`KismetMathLibrary.Lerp` 0.0 -10.0 _switcheffect)) false false))
      (:`Finished`
        (set `self.IsSolved` true)
        (`PrimitiveComponent.SetMaterial` (`self.Switch_Mesh`) 0 "/Game/Materials/M_Green.M_Green")
        (`KismetSystemLibrary.Delay` 0.2)
        (`PlayerController.SetViewTargetWithBlend` (`GameplayStatics.GetPlayerController` 0) (`self.Door`) 0.4 "VTBlend_Linear" 0.0 false)
        (`self.DisableInput` (`GameplayStatics.GetPlayerCharacter` 0) (`GameplayStatics.GetPlayerController` 0))
        (`KismetSystemLibrary.Delay` 0.2)
        (message `/Game/BluePrints/Door/BI_Door.Opening` (`self.Door`))))))

(fn `Opening`)

(fn `Solved`
  (returns (IsTrigger :type Boolean))
  (return (`self.IsSolved`)))

(fn `UserConstructionScript`)