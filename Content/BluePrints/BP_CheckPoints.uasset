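; BP_CheckPoints is a checkpoint actor that records a respawn-style transform when the player reaches it.
; On BeginPlay it casts the game mode to BP_ThirdPersonGameMode and caches the reference.
; When player character 0 overlaps its Box, it prints a debug string and writes its own location and rotation, at unit scale, to the game mode's LastCheckpointTransform.
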(event `self.ReceiveBeginPlay`
  (bind _asbp_third_person_game_mode (cast `/Game/ThirdPerson/Blueprints/BP_ThirdPersonGameMode` (`GameplayStatics.GetGameMode`)))
  (set `self.GameMode` _asbp_third_person_game_mode))

(event `self.Box.OnComponentBeginOverlap`
  (params (OverlappedComponent :type "PrimitiveComponent Object Reference") (OtherActor :type "Actor Object Reference") (OtherComp :type "PrimitiveComponent Object Reference") (OtherBodyIndex :type Integer) (bFromSweep :type Boolean) (SweepResult :type "HitResult Structure (by ref)"))
  (if (== OtherActor (`GameplayStatics.GetPlayerCharacter` 0))
    (`KismetSystemLibrary.PrintString` "checkpoint")
    (set `/Game/ThirdPerson/Blueprints/BP_ThirdPersonGameMode.LastCheckpointTransform` (`KismetMathLibrary.MakeTransform` (`self.K2_GetActorLocation`) (`self.K2_GetActorRotation`)) (`self.GameMode`))))

(fn `UserConstructionScript`)